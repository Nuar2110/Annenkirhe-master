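; Portal actor that teleports the VR pawn to linked portals through separate forward and backward triggers.
; On begin play, each side's widget shows the display name of its target portal.
; When the pawn's CameraCollision-tagged component enters a trigger, the pawn moves to the target's same-side trigger, offset downward.
; Before teleporting, it briefly disables both destination triggers to avoid an immediate bounce back.
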(event `self.ReceiveBeginPlay`
  (bind _asportal_text (cast `/Game/Widgets/Annenkhire/Portal_Text` (`WidgetComponent.GetUserWidgetObject` (`self.ForwardWidget`))))
  (`/Game/Widgets/Annenkhire/Portal_Text.ChangeText` _asportal_text (`KismetSystemLibrary.GetDisplayName` (`self.TargetPositionForward`)))
  (bind _asportal_text_2 (cast `/Game/Widgets/Annenkhire/Portal_Text` (`WidgetComponent.GetUserWidgetObject` (`self.BackwardWidget`))))
  (`/Game/Widgets/Annenkhire/Portal_Text.ChangeText` _asportal_text_2 (`KismetSystemLibrary.GetDisplayName` (`self.TargetPositionBackward`))))

(event `self.ReceiveTick`
  (params (DeltaSeconds :type "Float (single-precision)")))

(event `self.PortalTriggerForward.OnComponentBeginOverlap`
  (params (OverlappedComponent :type "PrimitiveComponent Object Reference") (OtherActor :type "Actor Object Reference") (OtherComp :type "PrimitiveComponent Object Reference") (OtherBodyIndex :type Integer) (bFromSweep :type Boolean) (SweepResult :type "HitResult Structure (by ref)"))
  (bind _asvrpawn (cast `/Game/Blueprints/VRPawn` OtherActor))
  (if (`ActorComponent.ComponentHasTag` OtherComp "CameraCollision")
    (`self.HideTriggers` (`self.TargetPositionForward`))
    (`/Game/Blueprints/VRPawn.TeleportActor` _asvrpawn (- (`SceneComponent.K2_GetComponentLocation` (`/Game/Blueprints/Portal.PortalTriggerForward` (`self.TargetPositionForward`))) (0.0 0.0 100.0)))))

(event `self.PortalTriggerBackward.OnComponentBeginOverlap`
  (params (OverlappedComponent :type "PrimitiveComponent Object Reference") (OtherActor :type "Actor Object Reference") (OtherComp :type "PrimitiveComponent Object Reference") (OtherBodyIndex :type Integer) (bFromSweep :type Boolean) (SweepResult :type "HitResult Structure (by ref)"))
  (bind _asvrpawn (cast `/Game/Blueprints/VRPawn` OtherActor))
  (if (`ActorComponent.ComponentHasTag` OtherComp "CameraCollision")
    (`self.HideTriggers` (`self.TargetPositionBackward`))
    (`/Game/Blueprints/VRPawn.TeleportActor` _asvrpawn (- (`SceneComponent.K2_GetComponentLocation` (`/Game/Blueprints/Portal.PortalTriggerBackward` (`self.TargetPositionBackward`))) (0.0 0.0 100.0)))))

(event `HideTriggers`
  (`PrimitiveComponent.SetCollisionEnabled` (`self.PortalTriggerForward`) "NoCollision")
  (`PrimitiveComponent.SetCollisionEnabled` (`self.PortalTriggerBackward`) "NoCollision")
  (`KismetSystemLibrary.Delay` 3.0)
  (`PrimitiveComponent.SetCollisionEnabled` (`self.PortalTriggerForward`) "QueryOnly")
  (`PrimitiveComponent.SetCollisionEnabled` (`self.PortalTriggerBackward`) "QueryOnly"))

(fn `Degree`
  (params (Vector1 :type "Vector Structure") (Vector2 :type "Vector Structure"))
  (returns (Float :type "Float (double-precision)"))
  (return (`KismetMathLibrary.DegAcos` (`KismetMathLibrary.Dot_VectorVector` (`KismetMathLibrary.Normal` Vector1) (`KismetMathLibrary.Normal` Vector2)))))

(fn `UserConstructionScript`)